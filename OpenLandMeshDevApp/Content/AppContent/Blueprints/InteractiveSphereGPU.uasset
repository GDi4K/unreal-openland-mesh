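; InteractiveSphereGPU is a procedural mesh actor set up as a sphere that reacts to player proximity.
; After animations update, it raises the GPU "Amplitude" parameter as the player character approaches.
; GetPolygonMesh supplies a cube, and OnModifyVertex normalizes vertices for spherical projection, adding a time-based radial sine wave outside the build pass.
; The vertex graph's radius and wave multipliers are all zero, with no visible read of Amplitude.
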(event `self.OnAfterAnimations`
  (`self.SetGPUScalarParameter` "Amplitude" (* (- 1.0 (`KismetMathLibrary.FMin` (/ (`KismetMathLibrary.VSize` (- (`self.K2_GetActorLocation` (`GameplayStatics.GetPlayerCharacter` 0)) (`self.K2_GetActorLocation`))) 1000.0) 1.0)) 10.0)))

(fn `GetPolygonMesh`
  (returns (ReturnValue :type "OpenLandMeshPolygonMeshProxy Object Reference"))
  (bind _returnvalue (`OpenLandMeshPolygonMeshProxy.MakeCubeMesh`))
  (return _returnvalue))

(fn `OnModifyVertex`
  (params (Payload :type "VertexModifierPayload Structure"))
  (returns (ReturnValue :type "VertexModifierResult Structure"))
  (bind _returnvalue (`KismetMathLibrary.Normal` Payload_Position))
  (bind _returnvalue_2 (* _returnvalue 0.0))
  (return (make `VertexModifierResult` (`KismetMathLibrary.SelectVector` _returnvalue_2 (+ _returnvalue_2 (* _returnvalue (* (`KismetMathLibrary.Sin` (+ (* (`KismetMathLibrary.Vector_Distance` _returnvalue_2) 0.0) (* Payload_TimeInSeconds 0.0))) 0.0))) Payload_bOnBuilding))))

(fn `UserConstructionScript`)
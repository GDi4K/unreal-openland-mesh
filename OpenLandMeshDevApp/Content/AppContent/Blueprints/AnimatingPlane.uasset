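; Procedural plane actor that animates as a radial sine-wave ripple.
; GetPolygonMesh builds a plane mesh and rotates it a quarter turn to supply the base geometry.
; OnModifyVertex offsets each vertex along Z by a sine of time and its distance from RootPosition, shaped by Speed, Frequency and Amplitude.
; The event graph and construction script are empty, so all behavior lives in these two functions.
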(fn `GetPolygonMesh`
  (returns (ReturnValue :type "OpenLandMeshPolygonMeshProxy Object Reference"))
  (bind _returnvalue (`OpenLandMeshPolygonMeshProxy.MakePlaneMesh`))
  (bind _returnvalue_2 (`OpenLandMeshPolygonMeshProxy.Transform` _returnvalue (`KismetMathLibrary.MakeTransform` (0.0 0.0 0.0) (struct :`Roll` -90.0))))
  (return _returnvalue_2))

(fn `OnModifyVertex`
  (params (Payload :type "VertexModifierPayload Structure"))
  (returns (ReturnValue :type "VertexModifierResult Structure"))
  (return (make `VertexModifierResult` (+ Payload_Position (* (0.0 0.0 1.0) (* (`KismetMathLibrary.Sin` (+ (* Payload_TimeInSeconds (`self.Speed`)) (* (`KismetMathLibrary.Vector_Distance` Payload_Position (`self.RootPosition`)) (`self.Frequency`)))) (`self.Amplitude`)))))))

(fn `UserConstructionScript`)